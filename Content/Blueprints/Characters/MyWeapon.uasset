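; Player weapon Blueprint that auto-fires Projectile_Rapid projectiles with sound while the trigger is held.
; PullTrigger uses a DoOnce to fire immediately and start a looping Fire timer, which ReleaseTrigger clears and resets.
; A CanShoot cooldown timer caps the actual fire rate independently of that loop.
; Firing on an empty magazine triggers a delayed reload, guarded by IsReloading on the cached MyCharacter, that refills the ammo.
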(event `self.ReceiveBeginPlay`
  (`|ExecutionSequence`
    (:`then_0`
      ;[1 1 1] Store the player
      (bind _asmy_character (cast `/Game/Blueprints/Characters/MyCharacter` (`GameplayStatics.GetPlayerPawn` 0)))
      (set `self.PlayerReference` _asmy_character))
    (:`then_1`
      ;[1 1 1] Normal Gun Setup
      (set `self.CurrentAmmo_N` (`self.AmmoCount_N`))
      (set `self.GunSound_N` "/Game/Sounds/GunSound.GunSound"))
    (:`then_2`
      (set `self.ProjectileCooldown` (/ 1.0 4.0)))))

(event `PullTrigger`
  ;[1 1 1] Pull & Release Trigger Custom Events
  (`/Engine/EditorBlueprintResources/StandardMacros.DoOnce` false :!label _label
    (:`Completed`
      (`self.Fire`)
      (`KismetSystemLibrary.K2_SetTimer` null "Fire" 0.1 true))))

(event `ReleaseTrigger`
  ;[1 1 1] Pull & Release Trigger Custom Events
  (`KismetSystemLibrary.K2_ClearTimer` null "Fire")
  (goto _label :!via `Reset`))

(event `Fire`
  (bind _currentammo_n (`self.CurrentAmmo_N`))
  ;[1 1 1] Fire Event
  (if (`self.CanShoot`)
    (`KismetSystemLibrary.K2_SetTimerDelegate` (delegate `CheckFire`) (`self.ProjectileCooldown`))
    (set `self.CanShoot` false)
    (if (> _currentammo_n 0)
      (set `self.CurrentAmmo_N` (- _currentammo_n 1))
      (`GameplayStatics.SpawnSoundAtLocation` "/Game/Sounds/GunSound.GunSound" (`self.K2_GetActorLocation`))
      (`|SpawnActorFromClass` "/Game/Blueprints/Characters/Projectile_Rapid.Projectile_Rapid_C" (`SceneComponent.K2_GetComponentToWorld` (`self.ProjectileSpawnPoint`)) "Undefined" "OverrideRootScale")
      (else
        (`self.ReloadWeapon`)))))

(event `CheckFire`
  ;[1 1 1] Fire Event
  (set `self.CanShoot` true))

(event `ReloadWeapon`
  ;[1 1 1] Reload Weapon Event
  (if (not (`Entity.IsReloading` (`self.PlayerReference`)))
    (set `Entity.IsReloading` true (`self.PlayerReference`))
    (`GameplayStatics.PlaySound2D` "/Game/Sounds/Reload.Reload")
    (`KismetSystemLibrary.Delay` 1.7)
    (set `Entity.IsReloading` false (`self.PlayerReference`))
    (set `self.CurrentAmmo_N` (`self.AmmoCount_N`))))

(fn `UserConstructionScript`)