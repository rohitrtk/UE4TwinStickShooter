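; MyEnemy is an enemy character for a twin-stick game that hurts the player on contact and awards score when killed.
; Overlapping MyCharacter starts a looping DamagePlayer timer at an interval of 1/DPS, cleared when the overlap ends.
; AffectHealth runs CalculateHealth; on death it increments TwinStickMode's score, ignores collision channels, detaches its controller, spawns an explosion, then destroys itself after a delay.
; The construction script tints a dynamic material with EnemyColour.
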(event `DamagePlayer`
  ;[1 1 1] Damage Player Event
  (`/Game/Blueprints/Characters/MyCharacter.AffectHealth` (`self.Player`) (`self.Damage`)))

(event `self.ReceiveActorEndOverlap`
  (params (OtherActor :type "Actor Object Reference"))
  ;[1 1 1] Collision Exit
  (if (== OtherActor (`self.Player`))
    (`KismetSystemLibrary.K2_ClearTimer` null "DamagePlayer")))

(event `self.ReceiveActorBeginOverlap`
  (params (OtherActor :type "Actor Object Reference"))
  ;[1 1 1] Collision Enter
  (bind _asmy_character (cast `/Game/Blueprints/Characters/MyCharacter` OtherActor))
  (set `self.Player` _asmy_character)
  (`KismetSystemLibrary.K2_SetTimer` null "DamagePlayer" (/ 1.0 (`self.DPS`)) true))

(event `/Game/Blueprints/Characters/iDamageable.AffectHealth`
  (params (Delta :type "Float (single-precision)"))
  (bind _capsulecomponent (`self.CapsuleComponent`))
  ;[1 1 1] Affect Health Event
  (`self.CalculateHealth` Delta)
  (if (`self.IsDead`)
    (bind _astwin_stick_mode (cast `/Game/Blueprints/TwinStickMode` (`GameplayStatics.GetGameMode`)))
    (`/Game/Blueprints/TwinStickMode.IncrementScore` _astwin_stick_mode (`self.ScoreValue`))
    (`PrimitiveComponent.SetCollisionResponseToChannel` _capsulecomponent "ECC_WorldDynamic" "ECR_Ignore")
    (`PrimitiveComponent.SetCollisionResponseToChannel` _capsulecomponent "ECC_Pawn" "ECR_Ignore")
    (`self.DetachFromControllerPendingDestroy`)
    (`|SpawnActorFromClass` "/Game/Blueprints/Explosion.Explosion_C" (`self.GetTransform`) "Undefined" "OverrideRootScale")
    (`KismetSystemLibrary.Delay` 3.0)
    (`self.K2_DestroyActor`)))

(fn `UserConstructionScript`
  (bind _returnvalue (`PrimitiveComponent.CreateDynamicMaterialInstance` (`self.Mesh`) 0 null))
  (bind _output_get (set `self.Dyn Mat` _returnvalue))
  (`MaterialInstanceDynamic.SetVectorParameterValue` _output_get "BodyColor" (`self.Enemy Colour`)))