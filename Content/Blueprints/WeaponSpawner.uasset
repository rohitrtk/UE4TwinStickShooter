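; Weapon spawner actor that spawns a MyWeapon_Rap at a random point inside its SpawnVolume box.
; BeginPlay fires StartWepTimer, which waits a short random delay and then spawns a single weapon.
; The new weapon is stored, flagged as FreshSpawn and given a ParentSpawner reference back to this spawner.
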(event `self.ReceiveBeginPlay`
  ;[1 1 1] Event BeginPlay
  (`self.StartWepTimer`))

(event `StartWepTimer`
  (bind _spawnvolume (`self.SpawnVolume`))
  ;[1 1 1] Event StartWepTimer
  (bind _output_get (set `self.WaitTime` (`KismetMathLibrary.RandomFloatInRange` 0.0 1.0)))
  (`KismetSystemLibrary.Delay` _output_get)
  (bind _returnvalue (`|SpawnActorFromClass` "/Game/Blueprints/Weapons/MyWeapon_Rap.MyWeapon_Rap_C" (`KismetMathLibrary.Conv_VectorToTransform` (`KismetMathLibrary.RandomPointInBoundingBox` (`SceneComponent.K2_GetComponentLocation` _spawnvolume) (`BoxComponent.GetScaledBoxExtent` _spawnvolume))) "Undefined" "OverrideRootScale"))
  (bind _output_get_2 (set `self.SpawnedWeapon` _returnvalue))
  (set `/Game/Blueprints/Weapons/MyWeapon.FreshSpawn` true _output_get_2)
  (set `/Game/Blueprints/Weapons/MyWeapon.ParentSpawner` self (`self.SpawnedWeapon`)))

(fn `UserConstructionScript`)